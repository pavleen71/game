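; Finish-line checkpoint for a kart race, a child Blueprint that detects when a lap is completed.
; When a kart overlaps its Box, it gathers every other BP_checkpoint and verifies that all are triggered.
; If they are, it fires the lap-completed event dispatcher.
; A separate ResetCheckpoints function clears every checkpoint's triggered flag, though nothing in this Blueprint calls it.
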(event `self.Box.OnComponentBeginOverlap`
  (params (OverlappedComponent :type "PrimitiveComponent Object Reference") (OtherActor :type "Actor Object Reference") (OtherComp :type "PrimitiveComponent Object Reference") (OtherBodyIndex :type Integer) (bFromSweep :type Boolean) (SweepResult :type "HitResult Structure (by ref)"))
  ; check if the overlap object is kart
  (bind _iskart (`self.iskart` OtherActor))
  (if _iskart
    ; call function and check if all previous checkpoints are passed
    (bind _lapcompleted (`self.ifallcheckstriggered`))
    (if _lapcompleted
      (`self.OnLapCompleted_0`))))

(fn `ifallcheckstriggered`
  (returns (LapCompleted :type Boolean))
  (locals (bLapcompleted :type Boolean) (checkpoint :type "Array of /Game/Blueprints/BP_checkpoint Object Reference"))
  (`|ExecutionSequence`
    (:`then_0`
      ; getting all the checkpoints and storing them in array
      (bind _outactors (`GameplayStatics.GetAllActorsOfClass` "/Game/Blueprints/BP_checkpoint.BP_checkpoint_C"))
      (bind _output_get (set `local.checkpoint` _outactors))
      (`KismetArrayLibrary.Array_RemoveItem` _output_get self))
    (:`then_1`
      ; getting the checkpoints and then iterating over it
      (set `local.bLapcompleted` true)
      (for _array_element (`local.checkpoint`)
        ; if checkpoints are not  triggered then lap is not completed and break the loop
        (if (not (`/Game/Blueprints/BP_checkpoint.checkpointTriger` _array_element))
          (set `local.bLapcompleted` false)
          (break))))
    (:`then_2`
      ; return the lap completed variable
      (return (`local.bLapcompleted`)))))

(fn `resetCheckpoints`
  ; getting the array of checkpoints ingame and reset to not passed after lap completed
  (bind _outactors (`GameplayStatics.GetAllActorsOfClass` "/Game/Blueprints/BP_checkpoint.BP_checkpoint_C"))
  (for _array_element _outactors
    (set `/Game/Blueprints/BP_checkpoint.checkpointTriger` false _array_element)))

(fn `UserConstructionScript`
  (`parent.UserConstructionScript`))