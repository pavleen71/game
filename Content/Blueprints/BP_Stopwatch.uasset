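; BP_Stopwatch is a simple stopwatch Blueprint that measures time elapsed since play began.
; Tick adds each frame's DeltaSeconds to Totaltime and prints the running total on screen under a fixed key, so the message updates in place.
; RecordeTime returns the current Totaltime; BeginPlay calls it but discards the result.
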(event `self.ReceiveBeginPlay`
  (`self.RecordeTime`))

(event `self.ReceiveTick`
  (params (DeltaSeconds :type "Float (single-precision)"))
  (bind _output_get (set `self.Totaltime` (+ DeltaSeconds (`self.Totaltime`))))
  (`KismetSystemLibrary.PrintString` (`KismetStringLibrary.Concat_StrStr` "T0tal Time; " (`KismetStringLibrary.Conv_DoubleToString` _output_get)) true true (struct :`G` 0.66 :`B` 1.0 :`A` 1.0) 2.0 "DeltaTime"))

(fn `RecordeTime`
  (returns (recordedTime :type "Float (double-precision)"))
  (return (`self.Totaltime`)))