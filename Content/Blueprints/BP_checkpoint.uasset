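; BP_checkpoint is an ordered checkpoint for the kart game, registering only when a kart passes it in sequence.
; On box overlap it checks for a BP_Kart, then sets its triggered flag and fires the OncheckpointTriggered dispatcher if its PreviousCheckpoint is triggered or unset.
; It binds to the game mode's lap-complete event on BeginPlay to clear that flag and print a message each lap.
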(event `self.ReceiveBeginPlay`
  (bind _asbp_kart_game_mode (cast `/Game/Template/Blueprints/BP_KartGameMode` (`GameplayStatics.GetGameMode`)))
  (add `/Game/Template/Blueprints/BP_KartGameMode.OnLapCompleteG` _asbp_kart_game_mode (delegate `CustomEvent`)))

(event `CustomEvent`
  (params (`Lap Number ` :type Integer))
  (set `self.checkpointTriger` false)
  (`KismetSystemLibrary.PrintString` "Lap completed" true true (struct :`R` 0.356538 :`G` 1.0 :`B` 0.277807 :`A` 1.0) 7.0))

(event `self.Box.OnComponentBeginOverlap`
  (params (OverlappedComponent :type "PrimitiveComponent Object Reference") (OtherActor :type "Actor Object Reference") (OtherComp :type "PrimitiveComponent Object Reference") (OtherBodyIndex :type Integer) (bFromSweep :type Boolean) (SweepResult :type "HitResult Structure (by ref)"))
  ; is overlap is kart
  (bind _iskart (`self.iskart` OtherActor))
  (if _iskart
    ; if previous checkpoint is ttriggered set checkpoint triger to true
    (bind _triggered (`self.previouscheckpointtrigerred`))
    (if _triggered
      (set `self.checkpointTriger` true)
      (`self.OncheckpointTriggered`))))

(fn `iskart`
  (params (actor :type "Actor Object Reference"))
  (returns (iskart :type Boolean))
  (cast `/Game/Template/Blueprints/BP_Kart` actor
    (:`then`
      ; return true is cast is cart
      (return true))
    (:`CastFailed`
      (return false))))

(fn `previouscheckpointtrigerred`
  (returns (triggered :type Boolean))
  (bind _previouscheckpoint (`self.previousCheckpoint`))
  (`/Engine/EditorBlueprintResources/StandardMacros.IsValid` _previouscheckpoint
    (:`Is Valid`
      (if (`/Game/Blueprints/BP_checkpoint.checkpointTriger` _previouscheckpoint)
        _
        (else
          (return false))))
    (:`Is Not Valid`
      _))
  (return true))

(fn `UserConstructionScript`)